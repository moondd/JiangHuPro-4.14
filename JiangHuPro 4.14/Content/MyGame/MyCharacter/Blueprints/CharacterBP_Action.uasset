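; Character Blueprint for melee combat: weapon equip and sheathing, attacks, blocking, damage and death.
; Right-hand weapon overlaps pass CanDamage, which filters by team type and ID and allows one hit per target until AttackOver clears the list.
; TargetIsBlocking checks stamina, block state and facing, triggering either a block montage or hit reaction; unblocked hits spawn effects and apply damage.
; AnyDamage reduces health, then calls empty death or survival hook functions.
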(event `self.ReceiveBeginPlay`
  (`parent.ReceiveBeginPlay`)
  (bind _ascharacter_anim (cast `/Game/MyGame/MyCharacter/Animations/CharacterAnim` (`SkeletalMeshComponent.GetAnimInstance` (`self.Mesh`))))
  (set `self.CharacterAnim` _ascharacter_anim))

(event `self.ReceiveTick`
  (params (DeltaSeconds :type "Float (single-precision)"))
  (bind _weapontrail (`self.WeaponTrail`))
  ;[1 1 1] WeaponsTrail
  (`parent.ReceiveTick` 0.0)
  (if (`|EnumEquality` (`self.CharacterState`) "NewEnumerator1")
    (`ActorComponent.SetActive` _weapontrail true false)
    (else
      (`ActorComponent.SetActive` _weapontrail false false))))

(event `self.R-Hand.OnComponentBeginOverlap`
  (params (OverlappedComponent :type "PrimitiveComponent Object Reference") (OtherActor :type "Actor Object Reference") (OtherComp :type "PrimitiveComponent Object Reference") (OtherBodyIndex :type Integer) (bFromSweep :type Boolean) (SweepResult :type "HitResult Structure (by ref)"))
  (bind _returnvalue (`self.K2_GetActorLocation` OtherActor))
  (bind _r_hand (`self.R-Hand`))
  (bind _returnvalue_2 (`SceneComponent.GetSocketLocation` _r_hand "EffectStart"))
  ;[1 1 1] 伤害
  (bind _candamage_ (`self.CanDamage?` OtherActor))
  (if _candamage_
    (bind (_isblocking_ _damage) (`self.TargetIsBlocking` OtherActor (`self.DamageState`)))
    (if (not _isblocking_)
      (`GameplayStatics.SpawnEmitterAttached` "/Game/MyGame/MyEffects/BeDamage_Normal.BeDamage_Normal" OtherComp "None" (- _returnvalue_2 (* (- _returnvalue_2 _returnvalue) 0.5)) (`KismetMathLibrary.MakeRotator` (+ (.roll (`SceneComponent.GetSocketRotation` _r_hand "EffectStart")) 90.0) (.pitch (`KismetMathLibrary.FindLookAtRotation` (`self.K2_GetActorLocation`) _returnvalue)) (.yaw (`KismetMathLibrary.FindLookAtRotation` (`self.K2_GetActorLocation`) _returnvalue))) "KeepWorldPosition")
      (`GameplayStatics.ApplyDamage` OtherActor _damage null self))))

(event `self.ReceiveAnyDamage`
  (params (Damage :type "Float (single-precision)") (DamageType :type "DamageType Object Reference") (InstigatedBy :type "Controller Object Reference") (DamageCauser :type "Actor Object Reference"))
  (bind `_当前气血` (`self.当前气血`))
  (set `self.当前气血` (- `_当前气血` Damage))
  (if (<= `_当前气血` 0.0)
    (set `self.CharacterState` "NewEnumerator5")
    (`self.角色死亡`)
    (`PrimitiveComponent.SetCollisionEnabled` (`self.CapsuleComponent`) "NoCollision")
    (else
      (`self.攻击后未死亡` DamageCauser))))

(fn `AttackBegin`
  (params (NewParam :type "/Game/MyGame/MyCharacter/Animations/Enum_DamageState Enum"))
  (bind _output_get (set `self.DamageState` NewParam))
  (`self.NeedManaToDamage` _output_get)
  (`self.SetCurrMana` (- 0.0 (`self.伤害值`)))
  (return))

(fn `AttackOver`
  (set `self.DamageState` "NewEnumerator4")
  (`KismetArrayLibrary.Array_Clear` (`self.AttackTargets`))
  (return))

(fn `BeDamage`
  (params (DamageState :type "/Game/MyGame/MyCharacter/Animations/Enum_DamageState Enum"))
  (set `/Game/MyGame/MyCharacter/Animations/CharacterAnim.BeDamageState` DamageState (`self.CharacterAnim`))
  (return))

(fn `CanDamage?`
  (params (OtherActor :type "Actor Object Reference"))
  (returns (`CanDamage?` :type Boolean))
  (bind _attacktargets (`self.AttackTargets`))
  (if (and (!= OtherActor self) (`|EnumInequality` (`self.DamageState`) "NewEnumerator4") (not (`KismetArrayLibrary.Array_Contains` _attacktargets OtherActor)))
    (bind _asmy_character_bp (cast `/Game/MyGame/MyCharacter/Blueprints/MyCharacterBP` OtherActor)
      (:`then`
        (if (and (`|EnumEquality` (`self.团体类型`) (`/Game/MyGame/MyCharacter/Blueprints/MyCharacterBP.团体类型` _asmy_character_bp)) (== (`self.团体ID`) (`/Game/MyGame/MyCharacter/Blueprints/MyCharacterBP.团体ID` _asmy_character_bp)))
          (return false)
          (else
            (switch `/Game/MyGame/GameData/TeamEnum` (`self.团体类型`)
              (:`NewEnumerator0`
                (bind `_团体类型` (`/Game/MyGame/MyCharacter/Blueprints/MyCharacterBP.团体类型` _asmy_character_bp))
                (if (or (`|EnumEquality` `_团体类型` "NewEnumerator1") (`|EnumEquality` `_团体类型` "NewEnumerator3")) :!label _label
                  _
                  (else
                    (return false))))
              (:`NewEnumerator4`
                (goto _label))
              (:`NewEnumerator1`
                _)
              (:`NewEnumerator2`
                (if (or (`|EnumEquality` `_团体类型` "NewEnumerator0") (`|EnumEquality` `_团体类型` "NewEnumerator3") (`|EnumEquality` `_团体类型` "NewEnumerator4"))
                  (return false)
                  (else
                    _)))
              (:`NewEnumerator3`
                _))
            (`KismetArrayLibrary.Array_Add` _attacktargets OtherActor)
            (return true))))
      (:`CastFailed`
        _)))
  (return false))

(fn `DamageIsBlocking`
  (params (DamageState :type "/Game/MyGame/MyCharacter/Animations/Enum_DamageState Enum") (Damage :type "Float (double-precision)"))
  (`self.SetCurrMana` Damage)
  (`self.PlayAnimMontage` self "/Game/MyGame/MyCharacter/Animations/Montage/Block.Block" 0.6 "Blockinig")
  (return))

(fn `NeedManaToDamage`
  (params (DamageState :type "/Game/MyGame/MyCharacter/Animations/Enum_DamageState Enum"))
  (returns (NeedManaToDamage :type "Float (double-precision)"))
  (`|ExecutionSequence`
    (:`then_0`
      (if (`|EnumEquality` DamageState "NewEnumerator0")
        (return -20.0)))))

(fn `SetCurrMana`
  (params (Value :type "Float (double-precision)"))
  (set `self.当前体力` (+ (`self.当前体力`) Value)))

(fn `SetEqip`
  (bind _weapontrail (`self.WeaponTrail`))
  (`SceneComponent.K2_AttachTo` (`self.R-Hand`) (`self.Mesh`) "Bip001-R-Hand-Socket" "SnapToTargetIncludingScale" true)
  (set `self.IsREqip?` true)
  (`SceneComponent.K2_AttachTo` _weapontrail (`self.R-Hand`) "None" "SnapToTargetIncludingScale" true)
  (`ParticleSystemComponent.BeginTrails` _weapontrail "EffectStart" "EffectOver" "ETrailWidthMode_FromFirst" 1.0)
  (return))

(fn `SetUnEquip`
  (`SceneComponent.K2_AttachTo` (`self.R-Hand`) (`self.L_Hand`) "Socket" "SnapToTargetIncludingScale" true)
  (set `self.IsREqip?` false)
  (set `self.IsLEqip?` true)
  (return))

(fn `TargetIsBlocking`
  (params (TargetActor :type "Actor Object Reference") (DamageState :type "/Game/MyGame/MyCharacter/Animations/Enum_DamageState Enum"))
  (returns (`IsBlocking?` :type Boolean) (Damage :type "Float (double-precision)"))
  (bind `_伤害值` (`self.伤害值`))
  (bind _ascharacter_bp_action (cast `/Game/MyGame/MyCharacter/Blueprints/CharacterBP_Action` TargetActor))
  (if (and (> (`/Game/MyGame/MyCharacter/Blueprints/MyCharacterBP.当前体力` _ascharacter_bp_action) 0.0) (`|EnumEquality` (`/Game/MyGame/MyCharacter/Blueprints/CharacterBP_Action.CharacterState` _ascharacter_bp_action) "NewEnumerator2") (< (`KismetMathLibrary.DegAcos` (`KismetMathLibrary.Dot_VectorVector` (`KismetMathLibrary.Normal` (- (`self.K2_GetActorLocation` self) (`self.K2_GetActorLocation` TargetActor))) (`self.GetActorForwardVector` TargetActor))) 90.0))
    (`self.DamageIsBlocking` _ascharacter_bp_action DamageState 0.0)
    (return true `_伤害值`)
    (else
      (`self.BeDamage` _ascharacter_bp_action DamageState)
      (return false `_伤害值`))))

(fn `UserConstructionScript`
  (`parent.UserConstructionScript`)
  (`self.SetUnEquip`))

(fn `攻击后未死亡`
  (params (`伤害来自Actor` :type "Actor Object Reference")))

(fn `角色死亡`)