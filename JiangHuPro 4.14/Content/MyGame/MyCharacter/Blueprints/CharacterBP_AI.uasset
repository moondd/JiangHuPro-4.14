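; AI-controlled character that reacts to being attacked and picks its dialogue from its relationship with the player.
; BeginPlay caches the player and AI controller.
; Surviving a hit sphere-traces for nearby CharacterBP_AI, writes the attacker to their blackboard 警戒Actor key, and raises a player attacker's 威胁值 (threat).
; 获取当前对话ID derives dialogue IDs from relationship, identity and both sides' 性向 (alignment); 更新AI与玩家互动关系 repeats alignment checks but changes nothing.
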(event `self.ReceiveBeginPlay`
  (`parent.ReceiveBeginPlay`)
  (bind _ascharacter_bp_player (cast `/Game/MyGame/MyCharacter/Blueprints/CharacterBP_Player` (`GameplayStatics.GetPlayerPawn` 0)))
  (set `self.玩家角色` _ascharacter_bp_player)
  (bind _returnvalue (`AIBlueprintHelperLibrary.GetAIController` self))
  (bind `_asaic_ai控制器` (cast `/Game/MyGame/MyCharacter/Blueprints/AICharacter/AIC_AI控制器` _returnvalue))
  (set `self.MyAIController` `_asaic_ai控制器`)
  (`self.更新AI与玩家互动关系`))

(event `self.ReceiveTick`
  (params (DeltaSeconds :type "Float (single-precision)"))
  (`parent.ReceiveTick` 0.0))

(event `self.攻击后未死亡`
  (params (`伤害来自Actor` :type "Actor Object Reference"))
  (`self.受到攻击后通知周围角色警戒目标` `伤害来自Actor`)
  (bind _ascharacter_bp_player (cast `/Game/MyGame/MyCharacter/Blueprints/CharacterBP_Player` `伤害来自Actor`))
  (bind _result (`/Engine/EditorBlueprintResources/StandardMacros.IncrementInt` (`/Game/MyGame/MyCharacter/Blueprints/CharacterBP_Player.威胁值` _ascharacter_bp_player))
    (:`  `
      (set `/Game/MyGame/MyCharacter/Blueprints/CharacterBP_Player.威胁值` _result _ascharacter_bp_player))))

(event `self.角色死亡`)

(fn `UserConstructionScript`
  (`parent.UserConstructionScript`))

(fn `受到攻击后通知周围角色警戒目标`
  (params (Actor :type "Actor Object Reference"))
  (locals (NewLocalVar_0 :type "Array of EObjectTypeQuery Enum"))
  (bind _returnvalue (`self.K2_GetActorLocation`))
  (bind _outhits (`KismetSystemLibrary.SphereTraceMultiForObjects` :`Start` _returnvalue :`End` (+ _returnvalue (0.0 0.0 15.0)) :`Radius` 1000.0 :`ObjectTypes` (`local.NewLocalVar_0`) :`bIgnoreSelf` false))
  (for _array_element _outhits
    (bind _ascharacter_bp_ai (cast `/Game/MyGame/MyCharacter/Blueprints/CharacterBP_AI` (`.HitActor` (`GameplayStatics.BreakHitResult` _array_element))))
    (`/Game/MyGame/MyCharacter/Blueprints/AICharacter/AIC_AI控制器.SetBlackboardActor` (`/Game/MyGame/MyCharacter/Blueprints/CharacterBP_AI.MyAIController` _ascharacter_bp_ai) Actor "警戒Actor"))
  (return))

(fn `更新AI与玩家互动关系`
  (bind _returnvalue (`KismetMathLibrary.Conv_ByteToInt` (`/Game/MyGame/MyCharacter/Blueprints/MyCharacterBP.性向` (`self.玩家角色`))))
  (switch `/Game/MyGame/MyCharacter/Blueprints/特殊关系Enum` (`self.AI与玩家特殊关系`)
    (:`NewEnumerator0`
      (switch `/Game/MyGame/MyCharacter/Blueprints/性向Enum` (`self.性向`)
        (:`NewEnumerator0`
          (if (not (> _returnvalue 1)) :!label _label
            (return)))
        (:`NewEnumerator1`
          (goto _label))
        (:`NewEnumerator2`
          (return))
        (:`NewEnumerator3`
          (if (not (< _returnvalue 2)) :!label _label_2
            (return)))
        (:`NewEnumerator4`
          (goto _label_2))))))

(fn `获取当前对话ID`
  (bind _returnvalue (`KismetMathLibrary.Conv_ByteToInt` (`/Game/MyGame/MyCharacter/Blueprints/MyCharacterBP.性向` (`self.玩家角色`))))
  (switch `/Game/MyGame/MyCharacter/Blueprints/特殊关系Enum` (`self.AI与玩家特殊关系`)
    (:`NewEnumerator1`
      (set `self.当前对话ID` (`KismetStringLibrary.Conv_StringToName` (`|GetEnumeratorNameAsString` (`self.AI与玩家特殊关系`))))
      (return))
    (:`NewEnumerator0`
      (switch `/Game/MyGame/MyCharacter/Blueprints/性向Enum` (`self.性向`)
        (:`NewEnumerator0`
          (if (> _returnvalue 1) :!label _label
            _
            (else
              (set `self.当前对话ID` (`self.身份`) :!label _label_2)
              (return))))
        (:`NewEnumerator1`
          (goto _label))
        (:`NewEnumerator2`
          (goto _label_2))
        (:`NewEnumerator3`
          (if (< _returnvalue 2) :!label _label_3
            (return)
            (else
              (goto _label_2))))
        (:`NewEnumerator4`
          (goto _label_3)))
      (return))))