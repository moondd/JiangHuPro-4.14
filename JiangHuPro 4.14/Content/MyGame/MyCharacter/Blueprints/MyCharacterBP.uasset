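; Modular character Blueprint for a martial-arts RPG, building appearance and combat stats from CharacterData.
; Construction links Body and Pants to the master pose and fills the skill list from fixed row "1", ignoring SkillID.
; BeginPlay loads clothing meshes from DataTables with random dark tints, then derives health, inner power, stamina and damage from attribute-scaled growth rates.
; The alignment setter (设置善恶值) is empty, its branch logic disconnected.
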(event `self.ReceiveBeginPlay`
  (`self.SetMesh`)
  (`self.SetProperty `)
  (`self.设置善恶值`))

(event `self.ReceiveTick`
  (params (DeltaSeconds :type "Float (single-precision)")))

(fn `SetMesh`
  (bind _body (`self.Body`))
  (bind _pants (`self.Pants`))
  (bind (`_姓` `_名` `_善恶` `_根骨` `_臂力` `_定力` `_体力` `_胆识` `_上装` `_下装`) (break `/Game/MyGame/GameData/CharacterDataStruct` (`self.CharacterData`)))
  (bind _returnvalue (`PrimitiveComponent.GetMaterial` _body 0))
  (bind _returnvalue_2 (`PrimitiveComponent.GetMaterial` _pants 0))
  (`|ExecutionSequence`
    (:`then_0`
      (bind _returnvalue_3 (`|GetDataTableRow` "/Game/MyGame/GameData/BodyDataTable.BodyDataTable" `_上装`)
        (:`then`
          (`SkinnedMeshComponent.SetSkinnedAssetAndUpdate` _body (`.Mesh_5_D3279C78497200213C21409F8E49A76C` (break `/Game/MyGame/GameData/EqipStruct` _returnvalue_3)) true)
          (bind _returnvalue_4 (`KismetMaterialLibrary.CreateDynamicMaterialInstance` _returnvalue _returnvalue))
          (`PrimitiveComponent.SetMaterial` (`self.Body`) 0 _returnvalue_4)
          (`MaterialInstanceDynamic.SetVectorParameterValue` _returnvalue_4 "ClothColor" (`KismetMathLibrary.MakeColor` (`KismetMathLibrary.RandomFloatInRange` 0.01 0.2) (`KismetMathLibrary.RandomFloatInRange` 0.01 0.2) (`KismetMathLibrary.RandomFloatInRange` 0.01 0.2))))))
    (:`then_1`
      (bind _returnvalue_5 (`|GetDataTableRow` "/Game/MyGame/GameData/PantsDataTable.PantsDataTable" `_下装`)
        (:`then`
          (`SkinnedMeshComponent.SetSkinnedAssetAndUpdate` _pants (`.Mesh_5_D3279C78497200213C21409F8E49A76C` (break `/Game/MyGame/GameData/EqipStruct` _returnvalue_5)) true)
          (bind _returnvalue_6 (`KismetMaterialLibrary.CreateDynamicMaterialInstance` _returnvalue_2 _returnvalue_2))
          (`PrimitiveComponent.SetMaterial` _pants 0 _returnvalue_6)
          (`MaterialInstanceDynamic.SetVectorParameterValue` _returnvalue_6 "ClothColor" (`KismetMathLibrary.MakeColor` (`KismetMathLibrary.RandomFloatInRange` 0.01 0.2) (`KismetMathLibrary.RandomFloatInRange` 0.01 0.2) (`KismetMathLibrary.RandomFloatInRange` 0.01 0.2))))))))

(fn `SetProperty `
  (bind (`_姓` `_名` `_善恶` `_根骨` `_臂力` `_定力` `_体力`) (break `/Game/MyGame/GameData/CharacterDataStruct` (`self.CharacterData`)))
  (`|ExecutionSequence`
    (:`then_0`
      (set `self.气血成长` (+ 1.2 (* (* `_根骨` 0.01) 1.2))))
    (:`then_1`
      (set `self.伤害成长` (+ 0.2 (* (* `_臂力` 0.01) 0.2))))
    (:`then_2`
      (set `self.内力成长` (+ 0.3 (* (* `_定力` 0.01) 0.3))))
    (:`then_3`
      (set `self.体力成长` (+ 0.1 (* (* `_体力` 0.01) 0.1)))
      (`|ExecutionSequence`
        (:`then_0`
          ;[1 1 1] 气血最大值
          (set `self.最大气血` (+ (+ (* (`self.外功`) (`self.气血成长`)) 120.0) (* `_根骨` 0.6))))
        (:`then_1`
          ;[1 1 1] 内力最大值
          (set `self.最大内力` (+ (+ (* (`self.内功`) (`self.内力成长`)) 30.0) (* `_定力` 0.15))))
        (:`then_2`
          ;[1 1 1] 体力最大值
          (set `self.最大体力` (+ (+ (* (`self.身法`) (`self.体力成长`)) 100.0) (* `_体力` 0.5))))
        (:`then_3`
          ;[1 1 1] 伤害值
          (set `self.伤害值` (+ (+ (* (`self.招式`) (`self.伤害成长`)) 20.0) (* `_臂力` 0.1)))
          (return))))))

(fn `SetSkillsStruct`
  (params (SkillID :type Integer))
  (bind _returnvalue (`|GetDataTableRow` "/Game/MyGame/MyCharacter/SkillsDataTable.SkillsDataTable" "1")
    (:`then`
      (set `self.当前技能列表` (`|MakeArray` _returnvalue _returnvalue (struct) (struct) (struct) (struct))))))

(fn `UserConstructionScript`
  (bind _mesh (`self.Mesh`))
  (`SkinnedMeshComponent.SetLeaderPoseComponent` (`self.Body`) _mesh)
  (`SkinnedMeshComponent.SetLeaderPoseComponent` (`self.Pants`) _mesh)
  (`self.SetSkillsStruct` 0))

(fn `设置善恶值`)